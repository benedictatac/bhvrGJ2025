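; BP_LightBomb is a throwable item that launches on spawn and explodes once on hit.
; BeginPlay impulses the item mesh along the first player's control rotation; construction sets the parent item's mesh, material and pickup effect.
; Explode plays a sound, spawns an effect, prints debug text and sets a short lifespan.
; The effect's location comes from GetActorOfClass, so it may follow another bomb instance instead of itself.
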(event EventBeginPlay
  (|CallParentFunction)
  (Physics|AddImpulse (Variables|Default|GetItemMesh) (* (Math|Vector|GetForwardVector (Pawn|GetControlRotation (Game|GetPlayerController 0) :!class /Script/Engine.Controller)) 1e+03) "None" true))

(event Collision|EventActorBeginOverlap
  (params (OtherActor :type Actor%20Object%20Reference))
  (|CallParentFunction OtherActor) ; This node is disabled and will not be called.\nDrag off pins to build functionality.
)

(event EventTick
  (params (DeltaSeconds :type Float%20%28single-precision%29))
  (|CallParentFunction DeltaSeconds) ; This node is disabled and will not be called.\nDrag off pins to build functionality.
)

(event Collision|EventHit
  (params (MyComp :type Primitive%20Component%20Object%20Reference) (Other :type Actor%20Object%20Reference) (OtherComp :type Primitive%20Component%20Object%20Reference) (bSelfMoved :type Boolean) (HitLocation :type Vector :default "0, 0, 0") (HitNormal :type Vector :default "0, 0, 0") (NormalImpulse :type Vector :default "0, 0, 0") (Hit :type Hit%20Result%20Structure%20%28by%20ref%29))
  (Utilities|FlowControl|DoOnce false
    (:Completed
      (CallFunction|Explode))))

(event EventExplode
  (bind _returnvalue (Actor|GetActorOfClass "BP_LightBomb_C"))
  (Audio|PlaySound2D "/Game/Items/sounds/explode_Cue.explode_Cue" 1.0 1.0 0.0 0 0)
  (Niagara|SpawnSystematLocation "/Game/Items/FX/FX_LightBombHit.FX_LightBombHit" (Transformation|GetWorldLocation (Variables|/Game/Items/BP_ItemParent.BP_ItemParent_C|GetItemMesh _returnvalue)))
  (Development|PrintString "BOOOOOM")
  (Actor|SetLifeSpan 1.0))

(fn ConstructionScript
  (Variables|Default|SetDisplayedMat "/Game/Items/Materials/BaseItemMaterial.BaseItemMaterial")
  (Variables|Default|SetDisplayedMesh "/Game/StarterContent/Shapes/Shape_Cylinder.Shape_Cylinder")
  (Variables|Default|SetPickupFX "/Game/Items/FX/FX_LightBombPickup.FX_LightBombPickup")
  (|CallParentFunction))