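; BP_EMP is a thrown EMP item, set up with its own mesh, material and pickup effect.
; On spawn it launches along the player's view; its first hit triggers Explode, with sound and Niagara effect.
; Explode finds a BP_EMP by class rather than using self, overlaps WorldDynamic actors around it, and makes StaticMesh-cast matches disappear.
; Hiding and timed destruction run inside that loop, only after a successful cast.
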(event EventBeginPlay
  (|CallParentFunction)
  (Physics|AddImpulse (Variables|Default|GetItemMesh) (* (Math|Vector|GetForwardVector (Pawn|GetControlRotation (Game|GetPlayerController 0) :!class /Script/Engine.Controller)) 1e+03) "None" true))

(event Collision|EventActorBeginOverlap
  (params (OtherActor :type Actor%20Object%20Reference))
  (|CallParentFunction OtherActor) ; This node is disabled and will not be called.\nDrag off pins to build functionality.
)

(event EventTick
  (params (DeltaSeconds :type Float%20%28single-precision%29))
  (|CallParentFunction DeltaSeconds) ; This node is disabled and will not be called.\nDrag off pins to build functionality.
)

(event Collision|EventHit
  (params (MyComp :type Primitive%20Component%20Object%20Reference) (Other :type Actor%20Object%20Reference) (OtherComp :type Primitive%20Component%20Object%20Reference) (bSelfMoved :type Boolean) (HitLocation :type Vector :default "0, 0, 0") (HitNormal :type Vector :default "0, 0, 0") (NormalImpulse :type Vector :default "0, 0, 0") (Hit :type Hit%20Result%20Structure%20%28by%20ref%29))
  (Utilities|FlowControl|DoOnce false
    (:Completed
      (CallFunction|Explode))))

(event EventExplode
  (bind _returnvalue (Actor|GetActorOfClass "BP_EMP_C"))
  (Audio|PlaySound2D "/Game/Items/sounds/explode_Cue.explode_Cue" 1.0 1.0 0.0 0 0)
  (Niagara|SpawnSystematLocation "/Game/Items/FX/FX_EMPHit.FX_EMPHit" (Transformation|GetWorldLocation (Variables|/Game/Items/BP_ItemParent.BP_ItemParent_C|GetItemMesh _returnvalue)))
  (bind _outactors (Collision|SphereOverlapActors (Transformation|GetWorldLocation (Variables|/Game/Items/BP_ItemParent.BP_ItemParent_C|GetItemMesh _returnvalue)) 1e+03 (Utilities|Array|MakeArray "ObjectTypeQuery2") 0))
  (for _array_element _outactors
    (bind _asstatic_mesh (Utilities|Casting|CastToStaticMesh _array_element))
    (Utilities|Array|Add (Variables|Default|GetAs%20Static%20Mesh) _asstatic_mesh)
    (Default|Disappear _asstatic_mesh)
    (Development|PrintString "EMP INBOUND")
    (Actor|SetLifeSpan 5.0)
    (Development|SetHiddeninGame (Variables|Default|GetItemMesh) true false)))

(fn ConstructionScript
  (Variables|Default|SetDisplayedMat "/Game/Items/Materials/M_EMP.M_EMP")
  (Variables|Default|SetDisplayedMesh "/Game/StarterContent/Shapes/Shape_Torus.Shape_Torus")
  (Variables|Default|SetPickupFX "/Game/Items/FX/FX_EMPPickup.FX_EMPPickup")
  (|CallParentFunction))